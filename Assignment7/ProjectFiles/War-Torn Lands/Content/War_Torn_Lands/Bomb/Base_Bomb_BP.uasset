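; Base bomb projectile Blueprint for War Torn Lands that spins while active and explodes on hit.
; BeginPlay derives a DataTable row name from its display name to set blast radius, power and cost, and reverses spin for player cannons.
; On hit it damages DamageInterface targets, plays a radius-scaled explosion flipbook, fires a radial impulse and ends the GameMode's turn.
; The delayed actor-destroy nodes are unconnected.
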(event `self.ReceiveTick`
  (params (DeltaSeconds :type "Float (single-precision)"))
  (bind _bomb (`self.Bomb`))
  ;[1 1 1] Rotate Bomb when spawned
  (`SceneComponent.K2_SetWorldRotation` _bomb (`KismetMathLibrary.ComposeRotators` (`SceneComponent.K2_GetComponentRotation` _bomb) (`KismetMathLibrary.MakeRotator` 0.0 (* DeltaSeconds (`self.RotationPerSec`)))) false false))

(event `self.ReceiveBeginPlay`
  (bind _cannon (`self.Cannon`))
  (bind _radialforce (`self.RadialForce`))
  ;[1 1 1] Use Data table values
  (bind _returnvalue (`|GetDataTableRow` "/Game/War_Torn_Lands/DataTables/DataTable_Bomb_Data.DataTable_Bomb_Data" (`KismetStringLibrary.Conv_StringToName` (`KismetArrayLibrary.Array_Get` (`KismetStringLibrary.ParseIntoArray` (`KismetSystemLibrary.GetDisplayName` self) "Bomb"))))
    (:`then`
      (bind _output_get (set `RadialForceComponent.Radius` (break `/Game/War_Torn_Lands/DataTables/Struct_Bomb_Data` _returnvalue) _radialforce))
      (set `self.ExplosionRadius` _output_get)
      (set `RadialForceComponent.ImpulseStrength` (`.Blast_Power_5_5CD0037A48498F97BC07DAB915024E3F` (break `/Game/War_Torn_Lands/DataTables/Struct_Bomb_Data` _returnvalue)) _radialforce)
      (set `self.Cost` (`.Cost_8_9AC5709D4B9846CD8F44A9BF79C9DF32` (break `/Game/War_Torn_Lands/DataTables/Struct_Bomb_Data` _returnvalue)))
      ;[1 1 1] Controls Bomb rotation direction
      (`/Engine/EditorBlueprintResources/StandardMacros.IsValid` _cannon
        (:`Is Valid`
          (if (`/Game/War_Torn_Lands/Cannon/Cannon.Player` _cannon)
            (set `self.RotationPerSec` (* (`self.RotationPerSec`) -1.0))))
        (:`Is Not Valid`
          (`/Game/War_Torn_Lands/Error_Message_Library.Error Message` "Cannon Var Not Valid" self))))
    (:`RowNotFound`
      (`/Game/War_Torn_Lands/Error_Message_Library.Error Message` "Bomb DataTable Row Not Found" self))))

(event `self.ReceiveHit`
  (params (MyComp :type "PrimitiveComponent Object Reference") (Other :type "Actor Object Reference") (OtherComp :type "PrimitiveComponent Object Reference") (bSelfMoved :type Boolean) (HitLocation :type "Vector Structure") (HitNormal :type "Vector Structure") (NormalImpulse :type "Vector Structure") (Hit :type "HitResult Structure (by ref)"))
  (bind _explosion_animation (`self.Explosion_Animation`))
  (bind _sphere (`self.Sphere`))
  (bind (_returnvalue_x _returnvalue_y _returnvalue_z) (`KismetMathLibrary.BreakVector` (`SceneComponent.K2_GetComponentLocation` _explosion_animation)))
  ;[1 1 1] Deals damage if other piece is destructable. If NOT Piece does not take damage
  (if (`KismetSystemLibrary.DoesImplementInterface` Other "/Game/War_Torn_Lands/DamageInterface.DamageInterface_C")
    (message `/Game/War_Torn_Lands/DamageInterface.Take Damage` Other))
  (`PrimitiveComponent.SetSimulatePhysics` _sphere false)
  (`PrimitiveComponent.SetCollisionEnabled` _sphere "NoCollision")
  ;[1 1 1] Explosion Flipbook Animation
  (`PaperFlipbookComponent.SetFlipbook` _explosion_animation "/Game/War_Torn_Lands/Bomb/Assets/Explosion/Explosion_Flipbook.Explosion_Flipbook")
  (`SceneComponent.K2_SetWorldLocation` _explosion_animation (`KismetMathLibrary.MakeVector` _returnvalue_x (+ _returnvalue_y 5.0) _returnvalue_z) false false)
  (`SceneComponent.SetWorldScale3D` _explosion_animation (`KismetMathLibrary.Conv_DoubleToVector` (/ (`self.ExplosionRadius`) 200.0)))
  (`PaperFlipbookComponent.SetLooping` _explosion_animation false)
  ;[1 1 1] Fire Impulse for Bomb
  (`ActorComponent.K2_DestroyComponent` (`self.Bomb`))
  (`RadialForceComponent.FireImpulse` (`self.RadialForce`))
  ;[1 1 1] End Turn
  (bind _asgame_mode_wtl (cast `/Game/War_Torn_Lands/GameMode_WTL` (`GameplayStatics.GetGameMode`))
    (:`then`
      (`/Game/War_Torn_Lands/GameMode_WTL.End_Turn` _asgame_mode_wtl))
    (:`CastFailed`
      (`/Game/War_Torn_Lands/Error_Message_Library.Error Message` "GM Cast Fail" self))))

(fn `UserConstructionScript`)