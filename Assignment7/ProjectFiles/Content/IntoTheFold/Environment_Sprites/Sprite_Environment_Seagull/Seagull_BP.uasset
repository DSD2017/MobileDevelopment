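; Environment seagull Blueprint that glides to a landing spot once the ship is docked, then plays idle animations.
; Tick interpolates the actor toward LandPos while ShipDocked is true, then triggers the animation change once on arrival.
; Change_Animation swaps the static Paper2D sprite for the SeaRat flipbook and starts a self-repeating loop.
; Each loop randomly picks turning or, more often, resting, waiting out the flipbook's duration.
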(event `self.ReceiveBeginPlay`
  (set `self.Original_Pos` (`self.K2_GetActorLocation`)))

(event `FlipbookReturn`
  (switch `int` (`KismetMathLibrary.RandomIntegerInRange` 0 4)
    (:`0`
      (`PaperFlipbookComponent.SetFlipbook` (`self.SeaRat`) "/Game/IntoTheFold/Environment_Sprites/Sprite_Environment_Seagull/Seagull_Turn_FB.Seagull_Turn_FB"))
    (:`1`
      (`PaperFlipbookComponent.SetFlipbook` (`self.SeaRat`) "/Game/IntoTheFold/Environment_Sprites/Sprite_Environment_Seagull/Seagull_Resting_FB.Seagull_Resting_FB" :!label _label))
    (:`2`
      (goto _label))
    (:`3`
      (goto _label))
    (:`4`
      (goto _label)))
  (`KismetSystemLibrary.Delay` (`PaperFlipbook.GetTotalDuration` (`PaperFlipbookComponent.GetFlipbook` (`self.SeaRat`))))
  (`self.FlipbookReturn` :!label _label_2))

(event `Change_Animation`
  (`SceneComponent.SetHiddenInGame` (`self.PaperSprite`) true false)
  (`SceneComponent.SetHiddenInGame` (`self.SeaRat`) false false)
  (goto _label_2))

(event `self.ReceiveTick`
  (params (DeltaSeconds :type "Float (single-precision)"))
  (if (`self.Ship_Docked`)
    (if (== (`self.K2_GetActorLocation`) (`self.Land_Pos`) :`ErrorTolerance` 0.1)
      (`/Engine/EditorBlueprintResources/StandardMacros.DoOnce` false
        (:`Completed`
          (`self.Change_Animation`)))
      (else
        (`self.K2_SetActorLocation` (`KismetMathLibrary.VInterpTo` (`self.K2_GetActorLocation`) (`self.Land_Pos`) DeltaSeconds 4.0) true)))))

(fn `UserConstructionScript`)